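; BP_GameMode is a game mode that periodically hands out random test items to players.
; A looping three-second timer, started on BeginPlay, runs GrantTestItems, which acts only with authority.
; For every BP_PlayerCharacter, DesGameState creates an item instance from a random pick of funny face, magic box or staff, which is auto-added to that character's inventory.
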(event `self.ReceiveBeginPlay`
  (`KismetSystemLibrary.K2_SetTimerDelegate` (delegate `GrantTestItems`) 3.0 true))

(event `GrantTestItems`
  (if (`self.HasAuthority`)
    (`KismetSystemLibrary.PrintString` "Auth" false)
    (bind _outactors (`GameplayStatics.GetAllActorsOfClass` "/Game/BaseGame/Player/BP_PlayerCharacter.BP_PlayerCharacter_C"))
    (for _array_element _outactors
      (bind _asdes_game_state (cast `DesGameState` (`GameplayStatics.GetGameState`)))
      (bind _returnvalue (`DesGameState.CreateItemInstance` _asdes_game_state (select `int` (`KismetMathLibrary.RandomInteger` 3) :`0` "/Game/BaseGame/Items/FunnyFace/ID_FunnyFace.ID_FunnyFace_C" :`1` "/Game/BaseGame/Items/MagicBox/ID_MagicBox.ID_MagicBox_C" :`2` "/Game/BaseGame/Items/Staff/ID_Staff.ID_Staff_C" :!type "DesItemData Class Reference")))
      (`DesItemContainerComponent.AddItemAuto` (`DesPlayerCharacter.Inventory` _array_element) _returnvalue))
    (else
      (`KismetSystemLibrary.PrintString` "NoAuth" false))))

(fn `UserConstructionScript`)